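; Lifestone is a checkpoint actor that updates the player's spawn point when touched.
; When the controlled pawn overlaps its Trigger, it plays a spark emitter at the stone and writes the SpawnPoint component's transform to ThirdPersonGameMode's SpawnTransform.
; A DoOnce gate, reset after a short delay, throttles re-triggering.
; The gate precedes the pawn check, so an overlap by any other actor closes it without a reset.
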(event OnComponentBeginOverlap(Trigger)
  (params (OverlappedComponent :type Primitive%20Component%20Object%20Reference) (OtherActor :type Actor%20Object%20Reference) (OtherComp :type Primitive%20Component%20Object%20Reference) (OtherBodyIndex :type Integer) (bFromSweep :type Boolean) (SweepResult :type Hit%20Result%20Structure%20%28by%20ref%29))
  (Utilities|FlowControl|DoOnce false :!label _label
    (:Completed
      (if (== OtherActor (Pawn|GetControlledPawn (Game|GetPlayerController 0)))
        (Effects|SpawnEmitteratLocation "/Game/StarterContent/Particles/P_Sparks.P_Sparks" (Transformation|GetWorldLocation (Variables|Default|GetLifestone)))
        (Variables|Default|SetLifestoneSpawnTransform (Transformation|GetWorldTransform (Variables|Default|GetSpawnPoint)))
        (bind _asthird_person_game_mode (Utilities|Casting|CastToThirdPersonGameMode (Game|GetGameMode)))
        (Variables|/Game/ThirdPersonBP/Blueprints/ThirdPersonGameMode.ThirdPersonGameMode_C|SetSpawn%20Transform _asthird_person_game_mode (Variables|Default|GetLifestoneSpawnTransform))
        (Utilities|FlowControl|Delay 1.0)
        (goto _label Reset)))))

(fn ConstructionScript)