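; PortalSystem is a portal that teleports the ThirdPersonCharacter to another teleporter instance's spawn point.
; Any valid actor entering OverlapCollision puts a PortalWidget on player 0's screen and starts a three-second delay.
; A sequence then removes the widget after a further short delay, while immediately moving the overlapping actor, if it is that character, to InstancedTeleporter's SpawnPoint location and rotation.
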(event OnComponentBeginOverlap(OverlapCollision)
  (params (OverlappedComponent :type Primitive%20Component%20Object%20Reference) (OtherActor :type Actor%20Object%20Reference) (OtherComp :type Primitive%20Component%20Object%20Reference) (OtherBodyIndex :type Integer) (bFromSweep :type Boolean) (SweepResult :type Hit%20Result%20Structure%20%28by%20ref%29))
  (bind _instancedteleporter (Variables|Default|GetInstancedTeleporter))
  (bind _spawnpoint (Variables|PortalSystem_C|GetSpawnPoint _instancedteleporter))
  (bind _returnvalue (Transformation|GetWorldTransform _spawnpoint))
  (Utilities|IsValid OtherActor
    (:Is%20Valid
      (bind _returnvalue_2 (UserInterface|CreateWidget "/Game/RPG_Game/Blueprints/PortalSystem/PortalWidget.PortalWidget_C" (Game|GetPlayerController 0)))
      (bind _output_get (Variables|Default|SetPortal%20Widget _returnvalue_2))
      (UserInterface|Viewport|AddtoViewport _output_get 0)
      (Utilities|FlowControl|Delay 3.0)
      (Utilities|FlowControl|Sequence
        (:then_0
          (Utilities|FlowControl|Delay 0.5)
          (Widget|RemovefromParent (Variables|Default|GetPortal%20Widget)))
        (:then_1
          (bind _asthird_person_character (Utilities|Casting|CastToThirdPersonCharacter OtherActor))
          (Transformation|Teleport _asthird_person_character (.location _returnvalue) (.rotation _returnvalue)))))))

(event EventBeginPlay)

(fn ConstructionScript)