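; ElysiumDropPortal is a trigger that announces the Elysium area name on screen when its collision volume is overlapped.
; The overlap is handled only on the Remote (non-authority) branch, where a short delay leads into a DoOnce gate.
; The gate creates an ElysiumTitleWidget, shows it for a few seconds, then removes it and resets after a further cooldown to prevent repeat announcements.
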(event OnComponentBeginOverlap(Collision)
  (params (OverlappedComponent :type Primitive%20Component%20Object%20Reference) (OtherActor :type Actor%20Object%20Reference) (OtherComp :type Primitive%20Component%20Object%20Reference) (OtherBodyIndex :type Integer) (bFromSweep :type Boolean) (SweepResult :type Hit%20Result%20Structure%20%28by%20ref%29))
  ;[1 1 1] This collision using Overlap Event to trigger the name of the area you have now entered!
  (Networking|SwitchHasAuthority
    (:Remote
      (Utilities|FlowControl|Delay 1.0)
      (Variables|Default|SetElysiumDrop (Variables|Default|GetElysiumDrop))
      (Variables|Default|SetElysiumEstablished (Variables|Default|GetElysiumEstablished))
      (Utilities|FlowControl|DoOnce false :!label _label
        (:Completed
          (bind _returnvalue (UserInterface|CreateWidget "/Game/RPG_Game/Blueprints/DestinationTitleAnnoucement/ElysiumTitleWidget.ElysiumTitleWidget_C" (Widget|GetOwningPlayer (Variables|Default|GetPLayerWidget))))
          (bind _output_get (Variables|Default|SetElysiumTitleVar _returnvalue))
          (UserInterface|Viewport|AddtoViewport _output_get 0)
          (Utilities|FlowControl|Delay 5.0)
          (Widget|RemovefromParent _output_get)
          (Utilities|FlowControl|Delay 1e+01)
          (goto _label Reset))))))

(fn ConstructionScript)